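; Multiplayer player controller that manages each player's UI, input, spawn rotation, respawn requests and session exit in PvP matches.
; Possession triggers local HUD and game-only input setup, then starts the BP_NecoArc pawn's begin play through the server.
; On spawn it retries each tick until game state and player state are cached, then flags the player ready.
; Events drive countdown, match timer, scoreboard and game-over screens, while a function shows the death menu.
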(event `SetSpawnRotation`
  (params (`New Rotation Z (Yaw)` :type "Float (single-precision)"))
  ;[1 1 1] Setting spawn rotation
  (`self.SetControlRotation` (`KismetMathLibrary.MakeRotator` 0.0 0.0 `New Rotation Z (Yaw)`)))

(event `Srv_StartBeginPlay`
  ;[1 1 1] Setting input mode to game only and removing all widgets
  (bind _asbp_neco_arc (cast `/Game/Characters/Heroes/Neco_Arc/BP_NecoArc` (`self.K2_GetPawn`) :!label _label))
  (`/Game/Characters/Heroes/Neco_Arc/BP_NecoArc.MC_BeginPlay` _asbp_neco_arc))

(event `MC_BeginPLay`
  ;[1 1 1] Setting input mode to game only and removing all widgets
  (if (`self.IsLocalPlayerController`)
    (`WidgetLayoutLibrary.RemoveAllWidgets`)
    (`self.UI_ShowInGameHUD`)
    (`WidgetBlueprintLibrary.SetInputMode_GameOnly` self)
    (set `self.bShowMouseCursor` false)
    (`/Engine/EditorBlueprintResources/ActorMacros.Switch Has Authority`
      (:`Authority`
        (goto _label))
      (:`Remote`
        (`self.Srv_StartBeginPlay`)))))

(event `EnableAllInput`
  ;[1 1 1] Enabling all inputs
  (`self.EnableInput` (`self.K2_GetPawn`) self))

(event `OnControllerSpawned`
  ;[1 1 1] Creating Game State and Player State Variables
  (bind _asbp_game_state (cast `/Game/Framework/BP_GameState` (`GameplayStatics.GetGameState`) :!label _label_2)
    (:`then`
      (set `self.BP_GameState` _asbp_game_state)
      (bind _asbp_player_state (cast `/Game/Framework/BP_PlayerState` (`self.PlayerState`) :!label _label_3)
        (:`then`
          (set `self.BP_PlayerState` _asbp_player_state)
          (set `self.IsPlayerReady` true))
        (:`CastFailed`
          (`KismetSystemLibrary.DelayUntilNextTick`)
          (goto _label_3))))
    (:`CastFailed`
      (`KismetSystemLibrary.DelayUntilNextTick`)
      (goto _label_2))))

(event `GameStartCountDown`
  ;[1 1 1] StartingCountdown
  (`/Game/Widgets/HUD/WB_IngameHUD.GameStartCountdown` (`self.WB_InGameHUD`)))

(event `UnHide_IngameHUD`
  ;[1 1 1] Unhiding in game hud
  (`Widget.SetVisibility` (`self.WB_InGameHUD`) "Visible"))

(event `EndClientSession`
  ;[1 1 1] Ending session for all clents
  (bind _asbp_game_instance (cast `/Game/Framework/BP_GameInstance` (`GameplayStatics.GetGameInstance`)))
  (set `/Game/Framework/BP_GameInstance.MP_IsPauseGameVisible` false _asbp_game_instance)
  (`DestroySessionCallbackProxy.DestroySession` self
    (:`then`
      (`GameplayStatics.OpenLevelBySoftObjectPtr` "/Game/Maps/Menu/MainMenu.MainMenu"))))

(event `self.ReceivePossess`
  (params (PossessedPawn :type "Pawn Object Reference"))
  ;[1 1 1] Calling beginplay on posses
  (`self.MC_BeginPLay`))

(event `HUD_StartMatch_PvP`
  ;[1 1 1] Starting PvP Match
  (`/Game/Widgets/HUD/WB_IngameHUD.GM_PvP_StartMatch` (`self.WB_InGameHUD`)))

(event `HUD_SetUpMatchTimer`
  (params (TimeLeftInSec :type Integer))
  (bind _wb_ingamehud (`self.WB_InGameHUD`))
  ;[1 1 1] Starting timer
  (`Widget.SetVisibility` (`/Game/Widgets/HUD/WB_IngameHUD.Text_MatchDuration` _wb_ingamehud) "Visible")
  (`/Game/Widgets/HUD/WB_IngameHUD.UpdateMatchTimer` _wb_ingamehud TimeLeftInSec))

(event `RespawnAfterDeath`
  ;[1 1 1] Respawning After Dying
  (bind _asbp_game_mode (cast `/Game/Framework/BP_GameMode` (`GameplayStatics.GetGameMode`)))
  (`/Game/Framework/BP_GameMode.Respawn After Dying` _asbp_game_mode self))

(event `UI_ShowGameOverScreen`
  (params (IsWinner :type Boolean) (IsScoreLimit :type Boolean) (IsTimeLimit :type Boolean))
  ;[1 1 1] Showing Game Over Screen
  (`WidgetLayoutLibrary.RemoveAllWidgets`)
  (bind _returnvalue (`|CreateWidget` "/Game/Widgets/UI/WB_GameOver.WB_GameOver_C" null IsWinner IsScoreLimit IsTimeLimit))
  (`UserWidget.AddToViewport` _returnvalue 0))

(event `Controller_DisableInput`
  ;[1 1 1] Disabling Input
  (`self.DisableInput` (`self.K2_GetPawn`) self))

(event `ClientToggleScoreBoard`
  (params (NewVisibility :type Boolean))
  ;[1 1 1] Toggling scoreboard
  (`self.UI_ToggleScoreBoard` NewVisibility))

(fn `UI_ShowInGameHUD`
  ;[1 1 1] Adding HUD to Viewport
  (`/Engine/EditorBlueprintResources/StandardMacros.IsValid` (`self.WB_InGameHUD`)
    (:`Is Valid`
      _)
    (:`Is Not Valid`
      (bind _returnvalue (`|CreateWidget` "/Game/Widgets/HUD/WB_IngameHUD.WB_IngameHUD_C" self))
      (bind _output_get (set `self.WB_InGameHUD` _returnvalue))))
  (`UserWidget.AddToViewport` _output_get 0))

(fn `UI_ShowPlayerDiedMenu`
  ;[1 1 1] Adding Player Died menu to a viewport
  (if (not (`self.IsGameOver`))
    (`/Engine/EditorBlueprintResources/StandardMacros.IsValid` (`self.WB_PlayerDiedMenu`)
      (:`Is Valid`
        _)
      (:`Is Not Valid`
        (bind _returnvalue (`|CreateWidget` "/Game/Widgets/UI/WB_PlayerDied.WB_PlayerDied_C"))
        (set `self.WB_PlayerDiedMenu` _returnvalue)))
    (`UserWidget.AddToViewport` (`self.WB_PlayerDiedMenu`) 0)
    (`WidgetBlueprintLibrary.SetInputMode_UIOnlyEx` self null)
    (set `self.bShowMouseCursor` true)
    (return)))

(fn `UI_ToggleScoreBoard`
  (params (NewVisibility :type Boolean))
  (bind _wb_scoreboard (`self.WB_ScoreBoard`))
  (if NewVisibility
    (`/Engine/EditorBlueprintResources/StandardMacros.IsValid` (`self.WB_ScoreBoard`)
      (:`Is Valid`
        _)
      (:`Is Not Valid`
        (bind _returnvalue (`|CreateWidget` "/Game/Widgets/UI/WB_ScoreBoard.WB_ScoreBoard_C" self))
        (set `self.WB_ScoreBoard` _returnvalue)))
    (`UserWidget.AddToViewport` (`self.WB_ScoreBoard`) 0)
    (else
      (`/Engine/EditorBlueprintResources/StandardMacros.IsValid` _wb_scoreboard
        (:`Is Valid`
          (`Widget.RemoveFromParent` _wb_scoreboard))
        (:`Is Not Valid`
          _))))
  (return))

(fn `UserConstructionScript`)