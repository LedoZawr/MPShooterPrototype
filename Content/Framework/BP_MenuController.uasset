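; Player controller for the multiplayer lobby menu, bridging each client's lobby UI and BP_Menu_GameMode.
; Initial setup loads or creates the saved player profile and sends it to the server, where the game mode updates the lobby.
; Ready state and chat go up through server events, while update events refresh names, readiness, level, mode and chat in WB_LobbyMenu.
; Other events show the lobby or load screen, or end the session and open the main menu.
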(event `self.ReceiveBeginPlay`
  ;[1 1 1] Setting input mode to UI only for Lobby Menu
  (if (`self.IsLocalController`)
    (set `self.bShowMouseCursor` true)
    (`WidgetBlueprintLibrary.SetInputMode_UIOnlyEx` self null)))

(event `EndClientSession`
  ;[1 1 1] Ending session for all clients (replicated)
  (`DestroySessionCallbackProxy.DestroySession` null
    (:`then`
      (`GameplayStatics.OpenLevelBySoftObjectPtr` "/Game/Maps/Menu/MainMenu.MainMenu"))))

(event `CreateLobbyMenu`
  ;[1 1 1] Creating lobby menu for all clients (replicated)
  (`self.UIShowLobbyMenu`))

(event `Create_LoadScreen`
  ;[1 1 1] Creating Load Screen for all clients (replicated)
  (`self.UIShowLoadScreen`))

(event `Initial_Setup`
  ;[1 1 1] Initial Setup (Replicated)
  (`self.LoadSavedProfile`)
  (set `self.IsProfileLoaded` true)
  (`self.Server_UpdateLobby` (`self.PlayerProfileInfo`)))

(event `Server_UpdateLobby`
  (params (`Player Profile` :type "/Game/SavedData/S_PlayerProfile Structure"))
  ;[1 1 1] Updating lobby on Server
  (set `self.PlayerProfileInfo` `Player Profile`)
  (bind _asbp_menu_game_mode (cast `/Game/Framework/BP_Menu_GameMode` (`GameplayStatics.GetGameMode`)))
  (`/Game/Framework/BP_Menu_GameMode.UpdateLobby` _asbp_menu_game_mode true true true true))

(event `Srv_UpdatePlayerReady`
  (params (IsReady :type Boolean))
  ;[1 1 1] Updating Player Ready
  (bind _asbp_menu_game_mode (cast `/Game/Framework/BP_Menu_GameMode` (`GameplayStatics.GetGameMode`)))
  (`/Game/Framework/BP_Menu_GameMode.SetPlayerReady` _asbp_menu_game_mode self IsReady))

(event `UpdatePlayerNames`
  (params (PlayerProfiles :type "Array of /Game/SavedData/S_PlayerProfile Structure"))
  (bind _wb_lobbymenu (`self.WB_LobbyMenu`))
  ;[1 1 1] Updating Player Names (Replicated)
  (`/Engine/EditorBlueprintResources/StandardMacros.IsValid` _wb_lobbymenu
    (:`Is Valid`
      (`/Game/Widgets/UI/WB_LobbyMenu.ClearPlayerNames` _wb_lobbymenu)
      (`/Game/Widgets/UI/WB_LobbyMenu.UpdatePlayerNames` _wb_lobbymenu PlayerProfiles))))

(event `UpdatePlayerReady`
  (params (IsPlayerReady :type "Array of Boolean"))
  (bind _wb_lobbymenu (`self.WB_LobbyMenu`))
  ;[1 1 1] Updating Player Ready
  (`/Engine/EditorBlueprintResources/StandardMacros.IsValid` _wb_lobbymenu
    (:`Is Valid`
      (`/Game/Widgets/UI/WB_LobbyMenu.UpdatePlayersReady` _wb_lobbymenu IsPlayerReady))))

(event `UpdateLevelSelection`
  (params (LevelRowName :type Name))
  (bind _wb_lobbymenu (`self.WB_LobbyMenu`))
  ;[1 1 1] Updating level selection for clients
  (`/Engine/EditorBlueprintResources/StandardMacros.IsValid` _wb_lobbymenu
    (:`Is Valid`
      (`/Game/Widgets/UI/WB_LobbyMenu.UpdateLevelSelection` _wb_lobbymenu LevelRowName))))

(event `UpdateChatBox`
  (params (Message :type Text))
  (bind _wb_lobbymenu (`self.WB_LobbyMenu`))
  ;[1 1 1] Updating chat box for server and clients
  (`/Engine/EditorBlueprintResources/StandardMacros.IsValid` _wb_lobbymenu
    (:`Is Valid`
      (`/Game/Widgets/UI/WB_LobbyMenu.AddChatMessage` _wb_lobbymenu Message))))

(event `Srv_SendChatMessage`
  (params (Message :type Text))
  ;[1 1 1] Updating chat box for server and clients
  (bind _asbp_menu_game_mode (cast `/Game/Framework/BP_Menu_GameMode` (`GameplayStatics.GetGameMode`)))
  (`/Game/Framework/BP_Menu_GameMode.SendChatMessage` _asbp_menu_game_mode Message))

(event `UpdateGameMode`
  (params (GameMode :type "/Game/Framework/E_GameModes Enum" :default "NewEnumerator2"))
  (bind _wb_lobbymenu (`self.WB_LobbyMenu`))
  ;[1 1 1] Updating Game Mode
  (`/Engine/EditorBlueprintResources/StandardMacros.IsValid` _wb_lobbymenu
    (:`Is Valid`
      (`/Game/Widgets/UI/WB_LobbyMenu.UpdateGameMode` _wb_lobbymenu (`|GetEnumeratorNameAsString` GameMode)))))

(fn `LoadSavedProfile`
  (locals (PlayerProfile_Slot :type String :default "PlayerProfile_Slot"))
  ;[1 1 1] Loading save game if exists and if not creating and loading
  (bind _returnvalue (`GameplayStatics.DoesSaveGameExist` (`local.PlayerProfile_Slot`)))
  (if (not _returnvalue)
    (bind _returnvalue_2 (`GameplayStatics.CreateSaveGameObject` "/Game/SavedData/SG_PlayerProfile.SG_PlayerProfile_C"))
    (`GameplayStatics.SaveGameToSlot` _returnvalue_2 (`local.PlayerProfile_Slot`)))
  (bind _returnvalue_3 (`GameplayStatics.LoadGameFromSlot` (`local.PlayerProfile_Slot`)))
  (bind _assg_player_profile (cast `/Game/SavedData/SG_PlayerProfile` _returnvalue_3))
  (set `self.PlayerProfileInfo` (`/Game/SavedData/SG_PlayerProfile.PlayerProfile` _assg_player_profile))
  (return))

(fn `UIShowLoadScreen`
  ;[1 1 1] Adding Lobby Menu to viewport while checking if valid
  (`WidgetLayoutLibrary.RemoveAllWidgets`)
  (`/Engine/EditorBlueprintResources/StandardMacros.IsValid` (`self.WB_LoadScreen`)
    (:`Is Valid`
      _)
    (:`Is Not Valid`
      (bind _returnvalue (`|CreateWidget` "/Game/Widgets/UI/WB_LoadScreen.WB_LoadScreen_C" self))
      (set `self.WB_LoadScreen` _returnvalue)))
  (`UserWidget.AddToViewport` (`self.WB_LoadScreen`) 0)
  (return))

(fn `UIShowLobbyMenu`
  ;[1 1 1] Adding Lobby Menu to viewport while checking if valid
  (`/Engine/EditorBlueprintResources/StandardMacros.IsValid` (`self.WB_LobbyMenu`)
    (:`Is Valid`
      _)
    (:`Is Not Valid`
      (bind _returnvalue (`|CreateWidget` "/Game/Widgets/UI/WB_LobbyMenu.WB_LobbyMenu_C" self))
      (set `self.WB_LobbyMenu` _returnvalue)))
  (`UserWidget.AddToViewport` (`self.WB_LobbyMenu`) 0)
  (return))

(fn `UserConstructionScript`)