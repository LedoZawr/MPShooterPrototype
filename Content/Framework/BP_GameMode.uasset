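; Game mode for multiplayer Free For All and Team Death Match, reading mode, match limits and expected player count from travel options.
; It waits for all players to be ready, spawns them at mode-tagged PlayerStarts, then runs a countdown.
; Respawns pick a random start with a short cooldown.
; In Free For All, a timer or kill score limit ends the match, showing results before server travel to Lobby.
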(event `self.HandleStartingNewPlayer`
  (params (NewPlayer :type "PlayerController Object Reference"))
  ;[1 1 1] Putting players to player spawn
  (bind _asbp_player_controller (cast `/Game/Framework/BP_PlayerController` NewPlayer))
  (`/Game/Framework/BP_PlayerController.OnControllerSpawned` _asbp_player_controller)
  (`KismetArrayLibrary.Array_Add` (`self.All_ConectedPlayers`) _asbp_player_controller)
  (if (`self.IsGameModeReady`) :!label _label
    (`self.UpdateGameStateInfo`)
    (bind _asbp_game_instance (cast `/Game/Framework/BP_GameInstance` (`GameplayStatics.GetGameInstance`)))
    (if (`/Game/Framework/BP_GameInstance.IsSoloGame` _asbp_game_instance)
      (`self.RestartPlayerAtPlayerStart` (`|GetArrayItem` (`self.All_ConectedPlayers`)) (`self.K2_FindPlayerStart` null (`KismetStringLibrary.Concat_StrStr` (`|GetEnumeratorNameAsString` (`self.GameMode`)) "_0")))
      (`self.LevelStart`)
      (elif (== (`self.Num_ExpectedPlayers`) (`KismetArrayLibrary.Array_Length` (`self.All_ConectedPlayers`)))
        (bind _all_playersready (`self.CountPlayersSpawned` :!label _label_2))
        (if _all_playersready
          (for (_array_element _array_index) (`self.All_ConectedPlayers`)
            (`self.RestartPlayerAtPlayerStart` _array_element (`self.K2_FindPlayerStart` _array_element (`KismetStringLibrary.Concat_StrStr` (`|GetEnumeratorNameAsString` (`self.GameMode`)) "_" (`KismetStringLibrary.Conv_IntToString` _array_index)))))
          (switch `/Game/Framework/E_GameModes` (`self.GameMode`)
            (:`NewEnumerator0`
              (`self.LvlStart_FreeForAll`)
              (`self.SetupRespawns`))
            (:`NewEnumerator1`
              (`self.LevelStart`)))
          (else
            (`KismetSystemLibrary.DelayUntilNextTick`)
            (goto _label_2)))))
    (else
      (`KismetSystemLibrary.DelayUntilNextTick`)
      (goto _label))))

(event `MatchTimer_Interval`
  ;[1 1 1] MatchTimer Interval
  (bind _result (`/Engine/EditorBlueprintResources/StandardMacros.DecrementInt` (`self.MatchDuration`))
    (:`  `
      (`/Game/Framework/BP_GameState.UpdateHUDMatchTimer` (`self.As BP Game State`) _result)
      (if (== (`self.MatchDuration`) 0)
        (`KismetSystemLibrary.PrintString` "Game Over" true true (struct :`R` 3.0 :`A` 1.0) 10.0)
        (`KismetSystemLibrary.K2_ClearAndInvalidateTimerHandle` (`self.MatchTimerHandle`))
        (bind _winner (`self.FindWinningPlayer`))
        (`self.GM_FFA_GameOver` false true _winner)))))

(event `self.ReceiveBeginPlay`
  ;[1 1 1] BeginPlay
  (`self.SetGameOptions` (`self.OptionsString`))
  (bind _asbp_game_state (cast `/Game/Framework/BP_GameState` (`GameplayStatics.GetGameState`)))
  (set `self.As BP Game State` _asbp_game_state)
  (set `self.IsGameModeReady` true))

(event `LevelStart`
  ;[1 1 1] Starting Level for all players
  (`KismetSystemLibrary.Delay` 0.2)
  (for _array_element (`self.All_ConectedPlayers`)
    (`/Game/Framework/BP_PlayerController.GameStartCountDown` _array_element))
  (`KismetSystemLibrary.Delay` 3.0)
  (for _array_element_2 (`self.All_ConectedPlayers`)
    (`/Game/Framework/BP_PlayerController.EnableAllInput` _array_element_2)))

(event `self.K2_OnLogout`
  (params (ExitingController :type "Controller Object Reference"))
  ;[1 1 1] Deleting player from an array if they left
  (bind _asbp_player_controller (cast `/Game/Framework/BP_PlayerController` ExitingController))
  (`KismetArrayLibrary.Array_RemoveItem` (`self.All_ConectedPlayers`) _asbp_player_controller)
  (`/Engine/EditorBlueprintResources/StandardMacros.DecrementInt` (`self.Num_ExpectedPlayers`)))

(event `RespawnPointCoolDown`
  (params (RespawnPoint :type String))
  ;[1 1 1] Cooldawn for respawn point
  (`KismetSystemLibrary.Delay` 4.0)
  (`BlueprintMapLibrary.Map_Add` (`self.All_RespawnPoints`) RespawnPoint))

(event `GM_FFA_GameOver`
  (params (IsScoreLimit :type Boolean) (IsTimeLimit :type Boolean) (Winner :type "/Game/Framework/BP_PlayerController Object Reference"))
  (for _array_element (`self.All_ConectedPlayers`)
    (set `/Game/Framework/BP_PlayerController.IsGameOver` true _array_element)
    (`/Game/Framework/BP_PlayerController.Controller_DisableInput` _array_element)
    (`/Game/Framework/BP_PlayerController.UI_ShowGameOverScreen` _array_element (== _array_element Winner) IsScoreLimit IsTimeLimit))
  (`KismetSystemLibrary.Delay` 3.0)
  (for _array_element_2 (`self.All_ConectedPlayers`)
    (`/Game/Framework/BP_PlayerController.ClientToggleScoreBoard` _array_element_2 true))
  (`KismetSystemLibrary.Delay` 8.0)
  (`KismetSystemLibrary.ExecuteConsoleCommand` "servertravel Lobby" (`GameplayStatics.GetPlayerController` 0)))

(event `LvlStart_FreeForAll`
  (bind _matchduration (`self.MatchDuration`))
  ;[1 1 1] Starting Free For All Mode
  (`KismetSystemLibrary.Delay` 1.0)
  (for _array_element (`self.All_ConectedPlayers`)
    (`/Game/Framework/BP_PlayerController.MC_BeginPLay` _array_element)
    (`/Game/Framework/BP_PlayerController.GameStartCountDown` _array_element)
    (if (> _matchduration 0)
      (`/Game/Framework/BP_PlayerController.HUD_SetUpMatchTimer` _array_element _matchduration)))
  (`KismetSystemLibrary.Delay` 3.0)
  (for _array_element_2 (`self.All_ConectedPlayers`)
    (`/Game/Framework/BP_PlayerController.EnableAllInput` _array_element_2)
    (`/Game/Framework/BP_PlayerController.HUD_StartMatch_PvP` _array_element_2))
  (if (> (`self.MatchDuration`) 0)
    (bind _returnvalue (`KismetSystemLibrary.K2_SetTimer` null "MatchTimer_Interval" 1.0 true))
    (set `self.MatchTimerHandle` _returnvalue)))

(fn `CountPlayersSpawned`
  (returns (`All PlayersReady` :type Boolean))
  (locals (Lcl_PlayersReady :type Integer))
  (for _array_element (`self.All_ConectedPlayers`)
    (if (`/Game/Framework/BP_PlayerController.IsPlayerReady` _array_element)
      (`/Engine/EditorBlueprintResources/StandardMacros.IncrementInt` (`local.Lcl_PlayersReady`))))
  (return (== (`KismetArrayLibrary.Array_Length` (`self.All_ConectedPlayers`)) (`local.Lcl_PlayersReady`))))

(fn `FindWinningPlayer`
  (returns (Winner :type "/Game/Framework/BP_PlayerController Object Reference"))
  (locals (Lcl_KillScores :type "Array of Integer"))
  (for (_array_element _array_index) (`self.All_ConectedPlayers`)
    (`KismetArrayLibrary.Array_Set` (`local.Lcl_KillScores`) _array_index (`/Game/Framework/BP_PlayerController.Kills` _array_element) true))
  (return (`|GetArrayItem` (`self.All_ConectedPlayers`) (`KismetMathLibrary.MaxOfIntArray` (`local.Lcl_KillScores`)))))

(fn `KilledPlayer`
  (params (Killer :type "/Game/Framework/BP_PlayerController Object Reference") (Victim :type "/Game/Framework/BP_PlayerController Object Reference"))
  (bind _result (`/Engine/EditorBlueprintResources/StandardMacros.IncrementInt` (`/Game/Framework/BP_PlayerController.Deaths` Victim))
    (:`  `
      (set `/Game/Framework/BP_PlayerState.Deaths` _result (`/Game/Framework/BP_PlayerController.BP_PlayerState` Victim))
      (bind _result_2 (`/Engine/EditorBlueprintResources/StandardMacros.IncrementInt` (`/Game/Framework/BP_PlayerController.Kills` Killer))
        (:`  `
          (bind _output_get (set `/Game/Framework/BP_PlayerState.Kills` _result_2 (`/Game/Framework/BP_PlayerController.BP_PlayerState` Killer)))
          (if (and (== _output_get (`self.ScoreLimit`)) (> (`self.ScoreLimit`) 0))
            (`self.GM_FFA_GameOver` true false (`local.Killer`))))))))

(fn `Respawn After Dying`
  (params (`Player Controller` :type "/Game/Framework/BP_PlayerController Object Reference"))
  (locals (Lcl_AllRespawnPoints :type "Array of String") (Lcl_PickedRespawnPoint :type String) (Lcl_LoopCount :type Integer))
  (bind _lcl_pickedrespawnpoint (`local.Lcl_PickedRespawnPoint`))
  (bind _returnvalue (`self.GetTransform` (`self.K2_FindPlayerStart` `Player Controller` (`local.Lcl_PickedRespawnPoint`))))
  ;[1 1 1] Finding Spawn Point and putting new controlled pawn there
  (bind _keys (`BlueprintMapLibrary.Map_Keys` (`self.All_RespawnPoints`)))
  (bind _output_get (set `local.Lcl_AllRespawnPoints` _keys))
  (set `local.Lcl_PickedRespawnPoint` (`KismetArrayLibrary.Array_Random` _output_get) :!label _label)
  (bind _result (`/Engine/EditorBlueprintResources/StandardMacros.IncrementInt` (`local.Lcl_LoopCount`))
    (:`  `
      (if (<= _result 10)
        (if (`BlueprintMapLibrary.Map_Find` (`self.All_RespawnPoints`) (`local.Lcl_PickedRespawnPoint`))
          (goto _label)
          (else
            _)))
      (`BlueprintMapLibrary.Map_Add` (`self.All_RespawnPoints`) _lcl_pickedrespawnpoint true)
      (`self.RespawnPointCoolDown` _lcl_pickedrespawnpoint)
      (`Controller.UnPossess` `Player Controller`)
      (`/Game/Framework/BP_PlayerController.SetSpawnRotation` `Player Controller` (.yaw (.rotation _returnvalue)))
      (bind _returnvalue_2 (`|SpawnActorFromClass` "/Game/Characters/Heroes/Neco_Arc/BP_NecoArc.BP_NecoArc_C" _returnvalue "Undefined" "MultiplyWithRoot" null null))
      (`Controller.Possess` `Player Controller` _returnvalue_2)
      (`/Game/Framework/BP_PlayerController.EnableAllInput` `Player Controller`)
      (return))))

(fn `SetGameOptions`
  (params (GameOptionString :type String))
  (switch `string` (`GameplayStatics.ParseOption` (`local.GameOptionString`) "GameMode")
    (:`FreeForAll`
      (set `self.GameMode` "NewEnumerator0"))
    (:`TeamDeathMatch`
      (set `self.GameMode` "NewEnumerator1")))
  (set `self.MatchDuration` (`KismetStringLibrary.Conv_StringToInt` (`GameplayStatics.ParseOption` (`local.GameOptionString`) "MatchDuration")))
  (set `self.ScoreLimit` (`KismetStringLibrary.Conv_StringToInt` (`GameplayStatics.ParseOption` (`local.GameOptionString`) "ScoreLimit")))
  (set `self.RespawnDelay` (`KismetStringLibrary.Conv_StringToInt` (`GameplayStatics.ParseOption` (`local.GameOptionString`) "RespawnDelay")))
  (set `self.Num_ExpectedPlayers` (`KismetStringLibrary.Conv_StringToInt` (`GameplayStatics.ParseOption` (`local.GameOptionString`) "NumConnectedPlayers")))
  (`KismetSystemLibrary.PrintString` (`GameplayStatics.ParseOption` (`local.GameOptionString`) "NumConnectedPlayers") true true (struct :`G` 0.66 :`B` 1.0 :`A` 1.0) 10.0)
  (`KismetSystemLibrary.PrintString` (`GameplayStatics.ParseOption` (`local.GameOptionString`) "GameMode"))
  (return))

(fn `SetupRespawns`
  (locals (Lcl_GameModeString :type String))
  (set `local.Lcl_GameModeString` (`|GetEnumeratorNameAsString` (`self.GameMode`)))
  (bind _outactors (`GameplayStatics.GetAllActorsOfClass` "/Script/Engine.PlayerStart"))
  (for _array_element _outactors
    (bind _returnvalue (`KismetStringLibrary.Conv_NameToString` (`PlayerStart.PlayerStartTag` _array_element)))
    (if (>= (`KismetStringLibrary.FindSubstring` _returnvalue (`local.Lcl_GameModeString`)) 0)
      (`BlueprintMapLibrary.Map_Add` (`self.All_RespawnPoints`) _returnvalue))))

(fn `UpdateGameStateInfo`
  (bind _as_bp_game_state (`self.As BP Game State`))
  (set `/Game/Framework/BP_GameState.CurrentGameMode` (`self.GameMode`) _as_bp_game_state)
  (set `/Game/Framework/BP_GameState.MatchDuration` (`self.MatchDuration`) _as_bp_game_state)
  (set `/Game/Framework/BP_GameState.ScoreLimit` (`self.ScoreLimit`) _as_bp_game_state))

(fn `UserConstructionScript`)