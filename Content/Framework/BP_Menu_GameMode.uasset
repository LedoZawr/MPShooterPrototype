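; Menu game mode that manages the multiplayer lobby: connected players, ready states, game mode selection and chat.
; Players entering the Lobby level are stored in index-matched controller and ready arrays and get a lobby menu; logout removes them.
; UpdateLobby uses flags to push names, level, readiness or mode to every BP_MenuController, also copying profiles into each BP_PlayerState.
; SendChatMessage relays messages to all controllers.
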(event `SetSelectedGameMode`
  (params (SelectedGameMode :type "/Game/Framework/E_GameModes Enum" :default "NewEnumerator2"))
  (set `self.SelectedGameMode` SelectedGameMode)
  (`self.UpdateLobby` false false false true))

(event `SetPlayerReady`
  (params (PlayerController :type "/Game/Framework/BP_MenuController Object Reference") (IsReady :type Boolean))
  ;[1 1 1] Updating Player
  (`KismetArrayLibrary.Array_Set` (`self.IsPlayerReady`) (`KismetArrayLibrary.Array_Find` (`self.All_ConnectedPlayers`) PlayerController) IsReady)
  (`self.UpdateLobby` false false true))

(event `self.HandleStartingNewPlayer`
  (params (NewPlayer :type "PlayerController Object Reference"))
  ;[1 1 1] Putting new players in the lobby and adding them to an array
  (bind _returnvalue (`GameplayStatics.GetCurrentLevelName` true))
  (switch `string` _returnvalue
    (:`Lobby`
      (bind _asbp_menu_controller (cast `/Game/Framework/BP_MenuController` NewPlayer))
      (bind _returnvalue_2 (`KismetArrayLibrary.Array_Add` (`self.All_ConnectedPlayers`) _asbp_menu_controller))
      (`KismetArrayLibrary.Array_Set` (`self.IsPlayerReady`) _returnvalue_2 false true)
      (`/Game/Framework/BP_MenuController.CreateLobbyMenu` _asbp_menu_controller)
      (`/Game/Framework/BP_MenuController.Initial_Setup` _asbp_menu_controller))))

(event `UpdateLobby`
  (params (PlayerNames :type Boolean) (LevelSelection :type Boolean) (PlayersReady :type Boolean) (GameMode :type Boolean))
  ;[1 1 1] Updating lobby, putting player names in arrays
  (if PlayerNames
    (`KismetArrayLibrary.Array_Clear` (`self.All_PlayerProfiles`))
    (for _array_element (`self.All_ConnectedPlayers`)
      (bind _playerprofileinfo (`/Game/Framework/BP_MenuController.PlayerProfileInfo` _array_element))
      (`KismetArrayLibrary.Array_Add` (`self.All_PlayerProfiles`) _playerprofileinfo)
      (bind _asbp_player_state (cast `/Game/Framework/BP_PlayerState` (`Controller.PlayerState` _array_element)))
      (set `/Game/Framework/BP_PlayerState.S_PlayerProfile` _playerprofileinfo _asbp_player_state)))
  (for _array_element_2 (`self.All_ConnectedPlayers`)
    (if PlayerNames
      (`/Game/Framework/BP_MenuController.UpdatePlayerNames` _array_element_2 (`self.All_PlayerProfiles`)))
    (if LevelSelection
      (`/Game/Framework/BP_MenuController.UpdateLevelSelection` _array_element_2 (`self.SelectedLevelName`)))
    (if PlayersReady
      (`/Game/Framework/BP_MenuController.UpdatePlayerReady` _array_element_2 (`self.IsPlayerReady`)))
    (if GameMode
      (`/Game/Framework/BP_MenuController.UpdateGameMode` _array_element_2 (`self.SelectedGameMode`)))))

(event `self.K2_OnLogout`
  (params (ExitingController :type "Controller Object Reference"))
  ;[1 1 1] Removing player names when leaving lobby
  (bind _asbp_menu_controller (cast `/Game/Framework/BP_MenuController` ExitingController))
  (bind _returnvalue (`KismetArrayLibrary.Array_Find` (`self.All_ConnectedPlayers`) _asbp_menu_controller))
  (`KismetArrayLibrary.Array_Remove` (`self.IsPlayerReady`) _returnvalue)
  (`KismetArrayLibrary.Array_Remove` (`self.All_ConnectedPlayers`) _returnvalue)
  (`self.UpdateLobby` true false true))

(fn `SendChatMessage`
  (params (Message :type Text))
  ;[1 1 1] Sending chat message
  (for _array_element (`self.All_ConnectedPlayers`)
    (`/Game/Framework/BP_MenuController.UpdateChatBox` _array_element Message)))

(fn `UserConstructionScript`)